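; BP_Vault is a storage vault whose cover slides open while the player pawn is in its parking spot.
; Overlapping ParkingSpot with BP_PlayerPawn plays the StorageDoor timeline, which drives the Cover's relative Y position, and leaving reverses it.
; A DebugOpenCover flag makes the construction script offset the cover along Y to preview it open in the editor.
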(event `Open Storage`
  (bind (_direction _storageposition) (`Timeline|StorageDoor` :!label _label)
    (:`Update`
      (`SceneComponent.K2_SetRelativeLocation` (`self.Cover`) (`KismetMathLibrary.MakeVector` 24.0 _storageposition 56.0) false false))))

(event `Close Storage`
  (goto _label :!via `Reverse`))

(event `self.ParkingSpot.OnComponentBeginOverlap`
  (params (OverlappedComponent :type "PrimitiveComponent Object Reference") (OtherActor :type "Actor Object Reference") (OtherComp :type "PrimitiveComponent Object Reference") (OtherBodyIndex :type Integer) (bFromSweep :type Boolean) (SweepResult :type "HitResult Structure (by ref)"))
  (cast `/Game/Blueprints/Player/BP_PlayerPawn` OtherActor)
  (`self.Open Storage`))

(event `self.ParkingSpot.OnComponentEndOverlap`
  (params (OverlappedComponent :type "PrimitiveComponent Object Reference") (OtherActor :type "Actor Object Reference") (OtherComp :type "PrimitiveComponent Object Reference") (OtherBodyIndex :type Integer))
  (cast `/Game/Blueprints/Player/BP_PlayerPawn` OtherActor)
  (`self.Close Storage`))

(fn `UserConstructionScript`
  (if (`self.bDebugOpenCover`)
    (`SceneComponent.K2_AddLocalOffset` (`self.Cover`) (0.0 134.0 0.0) false false)))