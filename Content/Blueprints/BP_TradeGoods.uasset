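; BP_TradeGoods is a clickable trade good that the player loads into a vehicle trunk and sells to a vault.
; Clicking its Cube while unloaded has the player vehicle load it into the trunk and sets IsLoaded.
; Clicking it while loaded has the vehicle sell it to its parked vault, then clears IsLoaded in a step marked as debug.
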(event `self.Cube.OnClicked`
  (params (TouchedComponent :type "PrimitiveComponent Object Reference") (ButtonPressed :type "Key Structure"))
  (bind _bp_playerpawn (`/Game/Blueprints/BPF_Common.GetPlayerVehicle`))
  (if (`self.IsLoaded`)
    (`/Game/Blueprints/Player/BP_PlayerPawn.Sell Actor To Vault` _bp_playerpawn (`/Game/Blueprints/Player/BP_PlayerPawn.Parked Vault Reference` _bp_playerpawn) self)
    ;[1 1 1] DEBUG
    (set `self.IsLoaded` false)
    (else
      (`/Game/Blueprints/Player/BP_PlayerPawn.Load Actor To Trunk` (`/Game/Blueprints/BPF_Common.GetPlayerVehicle`) self)
      (set `self.IsLoaded` true))))

(fn `UserConstructionScript`)