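; Base Blueprint for a trade good that the player buys and sells by clicking its cube.
; When not loaded, a click buys it at Price if money and a free vehicle slot allow, then loads it into the trunk.
; When loaded, a click sells it to the vehicle's parked vault if a slot is free, paying MaxPrice when its Type matches the vault's needed resource, otherwise Price.
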(event `self.Cube.OnClicked`
  (params (TouchedComponent :type "PrimitiveComponent Object Reference") (ButtonPressed :type "Key Structure"))
  (bind _bp_playerpawn (`/Game/Blueprints/BPF_Common.GetPlayerVehicle`))
  (bind _parked_vault_reference (`/Game/Blueprints/Player/BP_PlayerPawn.Parked Vault Reference` (`/Game/Blueprints/BPF_Common.GetPlayerVehicle`)))
  (if (`self.IsLoaded`)
    (`/Engine/EditorBlueprintResources/StandardMacros.IsValid` _parked_vault_reference
      (:`Is Valid`
        (if (`/Game/Blueprints/BPF_Common.GetFreeSlot` _parked_vault_reference)
          (if (== (`/Game/Blueprints/Trade/BP_Vault.NeededResource` _parked_vault_reference) (`self.Type`))
            (`/Game/Blueprints/BPF_Common.SellItem` (`self.MaxPrice`))
            (else
              (`/Game/Blueprints/BPF_Common.SellItem` (`self.Price`))))
          ;[1 1 1] Sell To Vault
          (`/Game/Blueprints/Player/BP_PlayerPawn.Sell Actor To Vault` _bp_playerpawn (`/Game/Blueprints/Player/BP_PlayerPawn.Parked Vault Reference` _bp_playerpawn) self)
          ;;[1 1 1] DEBUG
          (set `self.IsLoaded` false))))
    (elif (and (`/Game/Blueprints/BPF_Common.HasMoney` (`self.Price`)) (`/Game/Blueprints/BPF_Common.GetFreeSlot` (`/Game/Blueprints/BPF_Common.GetPlayerVehicle`)))
      (`/Game/Blueprints/BPF_Common.BuyItem` (`self.Price`))
      ;[1 1 1] Buy From vault
      (`/Game/Blueprints/Player/BP_PlayerPawn.Load Actor To Trunk` (`/Game/Blueprints/BPF_Common.GetPlayerVehicle`) self)
      (set `self.IsLoaded` true))))

(fn `UserConstructionScript`)