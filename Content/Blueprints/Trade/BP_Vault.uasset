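; BP_Vault is a trade storage point that opens when the player pawn parks in its spot and registers itself on that pawn.
; A timeline slides the cover open and reverses it when the pawn leaves.
; A looping timer with a randomized period rerolls the needed resource and, only while closed, replaces slot contents with a few goods.
; The spawned good type is mapped from the need, so it always differs from it.
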(event `Open Storage`
  ;[1 1 1] Overlap with car and animation
  (set `self.bIsOpen` true)
  (bind (_direction _storageposition) (`Timeline|StorageDoor` :!label _label)
    (:`Update`
      (`SceneComponent.K2_SetRelativeLocation` (`self.Cover`) (`KismetMathLibrary.MakeVector` 24.0 _storageposition 56.0) false false))))

(event `Close Storage`
  ;[1 1 1] Overlap with car and animation
  (set `self.bIsOpen` false)
  (goto _label :!via `Reverse`))

(event `self.ParkingSpot.OnComponentBeginOverlap`
  (params (OverlappedComponent :type "PrimitiveComponent Object Reference") (OtherActor :type "Actor Object Reference") (OtherComp :type "PrimitiveComponent Object Reference") (OtherBodyIndex :type Integer) (bFromSweep :type Boolean) (SweepResult :type "HitResult Structure (by ref)"))
  ;[1 1 1] Overlap with car and animation
  (bind _asbp_player_pawn (cast `/Game/Blueprints/Player/BP_PlayerPawn` OtherActor))
  (`self.Open Storage`)
  (set `/Game/Blueprints/Player/BP_PlayerPawn.Parked Vault Reference` self _asbp_player_pawn))

(event `self.ParkingSpot.OnComponentEndOverlap`
  (params (OverlappedComponent :type "PrimitiveComponent Object Reference") (OtherActor :type "Actor Object Reference") (OtherComp :type "PrimitiveComponent Object Reference") (OtherBodyIndex :type Integer))
  ;[1 1 1] Overlap with car and animation
  (bind _asbp_player_pawn (cast `/Game/Blueprints/Player/BP_PlayerPawn` OtherActor))
  (`self.Close Storage`)
  (set `/Game/Blueprints/Player/BP_PlayerPawn.Parked Vault Reference` null _asbp_player_pawn))

(event `Clear Storage`
  ;[1 1 1] Clean storage from all goods
  (if (not (`self.bIsOpen`))
    (for _array_element (`self.K2_GetComponentsByClass` "/Game/Blueprints/Trade/BP_Slot.BP_Slot_C")
      (bind _loadedgood (`/Game/Blueprints/Trade/BP_Slot.LoadedGood` _array_element))
      (`/Engine/EditorBlueprintResources/StandardMacros.IsValid` _loadedgood
        (:`Is Valid`
          (`self.K2_DestroyActor` _loadedgood)
          (`/Game/Blueprints/Trade/BP_Slot.Unload` _array_element))))))

(event `Update Needs Level`
  ;[1 1 1] Update Needs
  (set `self.NeededResource` (select `int` (`KismetMathLibrary.RandomIntegerInRange` 0 2) :`0` "NewEnumerator0" :`1` "NewEnumerator1" :`2` "NewEnumerator2" :!type "/Game/Blueprints/Trade/EGoodType Enum")))

(event `Spawn Resources In Storage`
  (bind (_returnvalue_location _returnvalue_rotation) (`KismetMathLibrary.BreakTransform` (`self.GetTransform`)))
  (bind (_hasfreeslot _slot) (`/Game/Blueprints/BPF_Common.GetFreeSlot` self))
  ;[1 1 1] Spawn Random Goods
  (for _ (range (+ (`KismetMathLibrary.RandomIntegerInRange` 1 3) 1))
    (if (`self.bIsOpen`)
      _
      (elif _hasfreeslot
        (bind _returnvalue (`|SpawnActorFromClass` (select `/Game/Blueprints/Trade/EGoodType` (`self.NeededResource`) :`NewEnumerator0` "/Game/Blueprints/Trade/BP_TradeGoods_Food.BP_TradeGoods_Food_C" :`NewEnumerator1` "/Game/Blueprints/Trade/BP_TradeGoods_Metal.BP_TradeGoods_Metal_C" :`NewEnumerator2` "/Game/Blueprints/Trade/BP_TradeGoods_Water.BP_TradeGoods_Water_C" :!type "Actor Class Reference") (`KismetMathLibrary.MakeTransform` _returnvalue_location _returnvalue_rotation) "AlwaysSpawn" "OverrideRootScale" null null))
        (bind _asbp_trade_goods_base (cast `/Game/Blueprints/Trade/BP_TradeGoods_Base` _returnvalue))
        (`/Game/Blueprints/Trade/BP_Slot.Load` _slot _asbp_trade_goods_base)))))

(event `Update Vault`
  ;[1 1 1] Logic Loop
  (`self.Clear Storage`)
  (`self.Update Needs Level`)
  (`self.Spawn Resources In Storage`))

(event `self.ReceiveBeginPlay`
  ;[1 1 1] Logic Loop
  (`KismetSystemLibrary.K2_SetTimerDelegate` (delegate `Update Vault`) (`KismetMathLibrary.RandomFloatInRange` 25.0 50.0) true)
  (`self.Update Vault`))

(fn `UserConstructionScript`
  (if (`self.bDebugOpenCover`)
    (`SceneComponent.K2_AddLocalOffset` (`self.Cover`) (0.0 134.0 0.0) false false)))