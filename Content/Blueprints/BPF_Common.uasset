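; Blueprint function library of shared helpers for cargo slots and the player's pawn.
; GetFreeSlot and FindItemInSlots linearly scan a target actor's BP_Slot components, returning the first empty slot or the one whose LoadedGood matches a given actor, with a success flag.
; GetPlayerVehicle returns player 0's pawn cast to BP_PlayerPawn.
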(fn `FindItemInSlots`
  (params (ActorToFind :type "/Game/Blueprints/BP_TradeGoods Object Reference") (Target :type "Actor Object Reference"))
  (returns (Found :type Boolean) (Slot :type "/Game/Blueprints/BP_Slot Object Reference"))
  (for _array_element (`Actor.K2_GetComponentsByClass` Target "/Game/Blueprints/BP_Slot.BP_Slot_C")
    (if (== ActorToFind (`/Game/Blueprints/BP_Slot.LoadedGood` _array_element))
      (return true _array_element)))
  (return false null))

(fn `GetFreeSlot`
  (params (Target :type "Actor Object Reference"))
  (returns (HasFreeSlot :type Boolean) (Slot :type "/Game/Blueprints/BP_Slot Object Reference"))
  (for _array_element (`Actor.K2_GetComponentsByClass` Target "/Game/Blueprints/BP_Slot.BP_Slot_C")
    (bind _isempty (`/Game/Blueprints/BP_Slot.IsEmpty` _array_element))
    (if _isempty
      (return _isempty _array_element)))
  (return false null))

(fn `GetPlayerVehicle`
  (returns (BP_PlayerPawn :type "/Game/Blueprints/Player/BP_PlayerPawn Object Reference"))
  (bind _asbp_player_pawn (cast `/Game/Blueprints/Player/BP_PlayerPawn` (`GameplayStatics.GetPlayerPawn` (`local.__WorldContext`))))
  (return _asbp_player_pawn))