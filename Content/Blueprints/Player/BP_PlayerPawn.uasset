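; Player vehicle pawn that drives and turns, rises and lands, takes collision damage and carries trade goods.
; Tick integrates axis input into clamped speed and local movement while locking the camera's world rotation; Shift raises top speed.
; W/S launch via a height Timeline, which Space reverses after stopping.
; Front/back overlaps cost health and invert motion; inventory events move goods between trunk and vault slots.
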(event `self.ReceiveTick`
  (params (DeltaSeconds :type "Float (single-precision)"))
  (bind _output_get (set `self.AccelerationSpeed` (`KismetMathLibrary.FClamp` (+ (`self.AccelerationSpeed`) (* (`self.AccelerationPower`) 2.0)) (`self.BackwardSpeed`) (`self.MaxSpeed`))))
  (`KismetSystemLibrary.PrintString` (`KismetStringLibrary.Conv_DoubleToString` _output_get) true true (struct :`G` 0.66 :`B` 1.0 :`A` 1.0) 0.0)
  (`self.K2_AddActorLocalTransform` (`KismetMathLibrary.MakeTransform` (`KismetMathLibrary.MakeVector` (* DeltaSeconds 1.0 (`self.AccelerationSpeed`))) (`KismetMathLibrary.MakeRotator` 0.0 0.0 (* DeltaSeconds (`self.TurnPower`) (`self.TurnSpeed`)))))
  (`SceneComponent.K2_SetWorldRotation` (`self.Camera`) (struct :`Pitch` -90.0) false false))

(event `Launch`
  (bind (_returnvalue_x _returnvalue_y) (`KismetMathLibrary.BreakVector` (`self.K2_GetActorLocation`)))
  (bind (_direction _height) (`Timeline|LaunchTimeline` :!label _label)
    (:`Update`
      (`self.K2_SetActorLocation` (`KismetMathLibrary.MakeVector` _returnvalue_x _returnvalue_y _height)))))

(event `Land`
  (goto _label :!via `Reverse`))

(event `InputAxis|Acceleration`
  (params (AxisValue :type "Float (single-precision)"))
  (set `self.AccelerationPower` AxisValue))

(event `Key|LeftShift`
  (params (Key :type "Key Structure"))
  (:`Pressed`
    (set `self.MaxSpeed` 1250.0))
  (:`Released`
    (set `self.MaxSpeed` 750.0)))

(event `InputAxis|Turn`
  (params (AxisValue :type "Float (single-precision)"))
  (set `self.TurnPower` AxisValue))

(event `Key|SpaceBar`
  (params (Key :type "Key Structure"))
  (:`Pressed`
    (set `self.AccelerationPower` 0.0)
    (set `self.AccelerationSpeed` 0.0)
    (`self.Land`)))

(event `Key|W`
  (params (Key :type "Key Structure"))
  (:`Pressed`
    (`self.Launch` :!label _label)))

(event `Key|S`
  (params (Key :type "Key Structure"))
  (:`Pressed`
    (goto _label)))

(event `self.FrontCollision.OnComponentBeginOverlap`
  (params (OverlappedComponent :type "PrimitiveComponent Object Reference") (OtherActor :type "Actor Object Reference") (OtherComp :type "PrimitiveComponent Object Reference") (OtherBodyIndex :type Integer) (bFromSweep :type Boolean) (SweepResult :type "HitResult Structure (by ref)"))
  ;[1 1 1] Damage
  (`self.ApplyDamageAndReverseMovement`))

(event `self.BackCollision.OnComponentBeginOverlap`
  (params (OverlappedComponent :type "PrimitiveComponent Object Reference") (OtherActor :type "Actor Object Reference") (OtherComp :type "PrimitiveComponent Object Reference") (OtherBodyIndex :type Integer) (bFromSweep :type Boolean) (SweepResult :type "HitResult Structure (by ref)"))
  ;[1 1 1] Damage
  (`self.ApplyDamageAndReverseMovement`))

(event `Load Actor To Trunk`
  (params (`Trade Good` :type "/Game/Blueprints/BP_TradeGoods_Base Object Reference"))
  (bind (_hasfreeslot _slot) (`/Game/Blueprints/BPF_Common.GetFreeSlot` self))
  (bind (_found _slot_2) (`/Game/Blueprints/BPF_Common.FindItemInSlots` `Trade Good` (`self.Parked Vault Reference`)))
  (`/Engine/EditorBlueprintResources/StandardMacros.IsValid` `Trade Good`
    (:`Is Valid`
      (if _hasfreeslot
        (`/Game/Blueprints/BP_Slot.Load` _slot `Trade Good`)
        (if _found
          (`/Game/Blueprints/BP_Slot.Unload` _slot_2))))))

(event `Sell Actor To Vault`
  (params (ParkedVault :type "/Game/Blueprints/BP_Vault Object Reference") (`Trade Good` :type "/Game/Blueprints/BP_TradeGoods_Base Object Reference"))
  (bind (_hasfreeslot _slot) (`/Game/Blueprints/BPF_Common.GetFreeSlot` ParkedVault))
  (bind (_found _slot_2) (`/Game/Blueprints/BPF_Common.FindItemInSlots` `Trade Good` self))
  (if (and _hasfreeslot _found)
    (`/Game/Blueprints/BP_Slot.Load` _slot `Trade Good`)
    (`/Game/Blueprints/BP_Slot.Unload` _slot_2)))

(fn `ApplyDamageAndReverseMovement`
  (`/Engine/EditorBlueprintResources/StandardMacros.DecrementFloat` (`self.Health`)
    (:`  `
      (set `self.AccelerationPower` (* (`self.AccelerationPower`) -1.0))
      (set `self.AccelerationSpeed` (* (`self.AccelerationSpeed`) -1.0)))))

(fn `UserConstructionScript`)